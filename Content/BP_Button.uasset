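; Floor-trigger button actor that makes a linked Nest spawn a turtle when the first-person character steps into it.
; On overlap with ButtonTrigger, it lowers PushedElem by a local offset and calls the push event.
; The push event checks that Nest is valid and uses ButtonPushed to spawn only once.
; The offset sits outside that guard, so each new overlap lowers the element again.
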(event `self.ReceiveBeginPlay`)

(event `self.ButtonTrigger.OnComponentBeginOverlap`
  (params (OverlappedComponent :type "PrimitiveComponent Object Reference") (OtherActor :type "Actor Object Reference") (OtherComp :type "PrimitiveComponent Object Reference") (OtherBodyIndex :type Integer) (bFromSweep :type Boolean) (SweepResult :type "HitResult Structure (by ref)"))
  (cast `/Game/FirstPersonCPP/Blueprints/FirstPersonCharacter` OtherActor)
  (`SceneComponent.K2_AddLocalOffset` (`self.PushedElem`) (0.0 0.0 -40.0) false false)
  (`self.PushButton_Event`))

(event `PushButton_Event`
  (if (and (`KismetSystemLibrary.IsValid` (`self.Nest`)) (not (`self.ButtonPushed`)))
    (set `self.ButtonPushed` true)
    (`/Game/BP_Nest.SpawnTurtle_Event` (`self.Nest`))))

(fn `UserConstructionScript`)