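; Turtle actor that travels in a straight line toward a target, alternating between a normal phase and an interval phase, each with its own speed and duration.
; Tick drives a timeline whose updates call TurtleAction to offset the turtle, and whose finish swaps the phase.
; The last step snaps to the target, updates the movement state on arrival, and can play a finish sound and hide particles.
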(event `self.ReceiveTick`
  (params (DeltaSeconds :type "Float (single-precision)"))
  (if (`self.IsTurtleMove`)
    (if (`self.FromStart`)
      (set `self.FromStart` false)
      (`TimelineComponent.SetTimelineLength` (`self.Timer`) (`self.ActionTime`))
      (`Timeline|Timer` :!via `SetNewTime` :!label _label
        (:`Update`
          (`self.TurtleAction`))
        (:`Finished`
          (if (`self.Phase`)
            (set `self.ActionSpeed` (`self.Speed`))
            (set `self.ActionTime` (`self.Time`))
            (else
              (set `self.ActionSpeed` (`self.IntervalSpeed`))
              (set `self.ActionTime` (`self.IntevalTime`))))
          (set `self.Phase` (not (`self.Phase`)))
          (set `self.FromStart` true)))
      (else
        (goto _label)))))

(fn `Init_TurtleInterval`
  (params (Speed :type "Float (double-precision)") (Target :type "/Game/Finish Object Reference") (IntervalSpeed :type "Float (double-precision)") (Time :type "Float (double-precision)") (IntervalTime :type "Float (double-precision)"))
  (`self.Init_turtleBase` Speed Target)
  (set `self.IntervalSpeed` IntervalSpeed)
  (set `self.Time` Time)
  (set `self.IntevalTime` IntervalTime)
  (set `self.ActionTime` (`self.Time`))
  (set `self.ActionSpeed` (`local.Speed`))
  (set `self.Direction` (`KismetMathLibrary.Normal` (- (`SceneComponent.K2_GetComponentLocation` (`/Game/Finish.DefaultSceneRoot` (`self.Target`))) (`SceneComponent.K2_GetComponentLocation` (`self.DefaultSceneRoot`))))))

(fn `Timer Handler`
  (locals (NewLocalVar_0 :type "TimelineComponent Object Reference"))
  (if (`KismetSystemLibrary.K2_IsValidTimerHandle` (struct))
    (if (not true)
      (if (`self.Phase`)
        (set `self.ActionSpeed` (`self.IntervalSpeed`))
        (set `self.ActionTime` (`self.IntevalTime`))
        (else
          (set `self.ActionSpeed` (`self.Speed`))
          (set `self.ActionTime` (`self.Time`))))
      (`KismetSystemLibrary.K2_SetTimer` self "TurtleAction" 0.1))))

(fn `TurtleAction`
  (locals (Distance :type "Vector Structure") (Delta :type "Vector Structure") (Offset :type "Vector Structure"))
  (set `local.Distance` (- (`SceneComponent.K2_GetComponentLocation` (`/Game/Finish.DefaultSceneRoot` (`self.Target`))) (`SceneComponent.K2_GetComponentLocation` (`self.DefaultSceneRoot`))))
  (set `local.Delta` (* (`self.Direction`) (`self.ActionSpeed`)))
  (if (> (`KismetMathLibrary.VSize` (`local.Distance`)) (`KismetMathLibrary.VSize` (`local.Delta`)))
    (`SceneComponent.K2_AddWorldOffset` (`self.DefaultSceneRoot`) (`local.Delta`) false false)
    (else
      (`SceneComponent.K2_AddWorldOffset` (`self.DefaultSceneRoot`) (`local.Distance`) false false)
      (bind _returnvalue (`self.IsTurtleArived`))
      (`self.SetTurtleMove` (not _returnvalue))
      (if (`self.isFinished`)
        (`GameplayStatics.PlaySound2D` "/Game/FinishSound.FinishSound" 1.0 1.0 0.0 null null false)
        (set `self.isFinished` false)
        (`SceneComponent.SetVisibility` (`self.ParticleSystem`) false false)))))

(fn `UserConstructionScript`)