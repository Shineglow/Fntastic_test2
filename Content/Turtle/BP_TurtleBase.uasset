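; BP_TurtleBase is a turtle actor that travels in a straight line toward a target actor set at initialization.
; While moving, each Tick offsets the root by a fixed Speed step, not scaled by delta time, snapping onto the target on the last step.
; That step checks X/Y arrival to call FinishArived and stop movement, plays a finish sound and hides particles.
; SetTurtleMove mirrors the moving flag to the TurtleActions anim instance.
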(event `self.ReceiveTick`
  (params (DeltaSeconds :type "Float (single-precision)"))
  (if (`self.IsTurtleMove`)
    (`self.TurtleAction`)))

(fn `Init_turtleBase`
  (params (Speed :type "Float (double-precision)") (Target :type "/Game/Finish Object Reference"))
  (set `self.Speed` Speed)
  (set `self.Target` Target))

(fn `IsTurtleArived`
  (returns (ReturnValue :type Boolean))
  (bind (_returnvalue_x _returnvalue_y) (`KismetMathLibrary.BreakVector` (`SceneComponent.K2_GetComponentLocation` (`self.DefaultSceneRoot`))))
  (bind (_returnvalue_x_2 _returnvalue_y_2) (`KismetMathLibrary.BreakVector` (`SceneComponent.K2_GetComponentLocation` (`/Game/Finish.DefaultSceneRoot` (`self.Target`)))))
  (if (`KismetMathLibrary.NearlyEqual_FloatFloat` (+ (- _returnvalue_x_2 _returnvalue_x) (- _returnvalue_y_2 _returnvalue_y)) 0.0 0.001)
    (`self.FinishArived`)
    (return true)
    (else
      (return false))))

(fn `SetTurtleMove`
  (params (IsMove :type Boolean))
  (set `self.IsTurtleMove` IsMove)
  (bind _asturtle_actions (cast `/Game/Turtle/TurtleActions` (`SkeletalMeshComponent.GetAnimInstance` (`self.SkeletalMesh`))))
  (set `/Game/Turtle/TurtleActions.IsTurtleMove` (`self.IsTurtleMove`) _asturtle_actions))

(fn `TurtleAction`
  (locals (Distance :type "Vector Structure" :default (0.0 0.0 0.0)) (Delta :type "Vector Structure" :default (0.0 0.0 0.0)) (Offset :type "Vector Structure"))
  (bind _output_get (set `local.Distance` (- (`SceneComponent.K2_GetComponentLocation` (`/Game/Finish.DefaultSceneRoot` (`self.Target`))) (`SceneComponent.K2_GetComponentLocation` (`self.DefaultSceneRoot`)))))
  (set `local.Delta` (* (`KismetMathLibrary.Normal` _output_get) (`self.Speed`)))
  (if (> (`KismetMathLibrary.VSize` (`local.Distance`)) (`KismetMathLibrary.VSize` (`local.Delta`)))
    (`SceneComponent.K2_AddWorldOffset` (`self.DefaultSceneRoot`) (`local.Delta`) false false)
    (else
      (`SceneComponent.K2_AddWorldOffset` (`self.DefaultSceneRoot`) (`local.Distance`) false false)
      (bind _returnvalue (`self.IsTurtleArived`))
      (`self.SetTurtleMove` (not _returnvalue))
      (`GameplayStatics.PlaySound2D` "/Game/FinishSound.FinishSound" 1.0 1.0 0.0 null null false)
      (`SceneComponent.SetVisibility` (`self.ParticleSystem`) false false))))

(fn `UserConstructionScript`)