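; Nest actor that spawns a turtle, either base or interval type, and sends it moving toward a Finish target.
; SpawnTurtle_Event shows a magic circle, then a two-second timer calls SpawnTurtleFunc, which spawns only when no valid turtle exists.
; The spawn function initializes movement settings by type, starts the turtle, plays a sound, hides the circle and binds to the turtle's finish-arrival event.
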(event `SpawnTurtle_Event`
  (`SceneComponent.SetVisibility` (`self.P_ky_magicCircle1`) true false)
  (`KismetSystemLibrary.K2_SetTimer` null "SpawnTurtleFunc" 2.0))

(fn `SpawnTurtleFunc`
  (if (not (`KismetSystemLibrary.IsValid` (`self.Turtle`)))
    (switch `/Game/TurtleType` (`self.Type`)
      (:`NewEnumerator0`
        (bind _returnvalue (`|SpawnActorFromClass` "/Game/Turtle/BP_TurtleBase.BP_TurtleBase_C" (`KismetMathLibrary.MakeTransform` (`self.SpawnPos`)) "Undefined" "OverrideRootScale" null null))
        (bind _output_get (set `self.Turtle` _returnvalue))
        (`/Game/Turtle/BP_TurtleBase.Init_turtleBase` _output_get (`self.TurtleInitialSpeed`) (`self.Finish`))
        (`/Game/Turtle/BP_TurtleBase.SetTurtleMove` (`self.Turtle`) true))
      (:`NewEnumerator1`
        (bind _returnvalue_2 (`|SpawnActorFromClass` "/Game/Turtle/BP_TurtleInterval.BP_TurtleInterval_C" (`KismetMathLibrary.MakeTransform` (`self.SpawnPos`)) "Undefined" "OverrideRootScale" null null))
        (bind _output_get_2 (set `self.Turtle` _returnvalue_2))
        (bind _asbp_turtle_interval (cast `/Game/Turtle/BP_TurtleInterval` _output_get_2))
        (`/Game/Turtle/BP_TurtleInterval.Init_TurtleInterval` _asbp_turtle_interval (`self.TurtleInitialSpeed`) (`self.Finish`) (`self.IntervalSpeed`) (`self.Time`) (`self.IntervalTime`))
        (`/Game/Turtle/BP_TurtleBase.SetTurtleMove` (`self.Turtle`) true)))
    (`GameplayStatics.PlaySound2D` "/Game/ShootSound.ShootSound" 1.0 1.0 0.0 null null)
    (`SceneComponent.SetVisibility` (`self.P_ky_magicCircle1`) false false)
    (add `/Game/Turtle/BP_TurtleBase.FinishArived` (`self.Turtle`) (`|CreateDelegate` (`self.Finish`) :!event `Fire`))))

(fn `UserConstructionScript`)