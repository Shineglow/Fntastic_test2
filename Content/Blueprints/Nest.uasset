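; Nest actor that spawns turtles, each launched with a particle burst and a loud shoot sound.
; SpawnOneTurtle plays the effects, spawns a Turtle_BP at the nest's root location and initializes it with the EndPoint actor's location, speed and move scale.
; A two-second timer calls StopEffect to deactivate the particles, which are also deactivated when the system finishes.
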(event `self.ParticleSystem.OnSystemFinished`
  (params (PSystem :type "ParticleSystemComponent Object Reference"))
  (`ActorComponent.Deactivate` PSystem))

(fn `PlayEffects`
  (`ActorComponent.Activate` (`self.ParticleSystem`) true)
  (`GameplayStatics.PlaySoundAtLocation` "/Game/Sounds/ShootSound.ShootSound" (`SceneComponent.K2_GetComponentLocation` (`self.DefaultSceneRoot`)) (struct) 30.0 1.0 0.0 null null self)
  (`KismetSystemLibrary.K2_SetTimer` self "StopEffect" 2.0))

(fn `SpawnOneTurtle`
  (`self.PlayEffects`)
  (bind _returnvalue (`|SpawnActorFromClass` "/Game/Blueprints/Turtle_BP.Turtle_BP_C" (`KismetMathLibrary.MakeTransform` (`SceneComponent.K2_GetComponentLocation` (`self.DefaultSceneRoot`))) "Undefined" "OverrideRootScale" null null))
  (`TurtleBase.InitTurtle` _returnvalue (`self.K2_GetActorLocation` (`self.EndPoint`)) (`self.Speed`) (`self.Move Scale`)))

(fn `StopEffect`
  (`ActorComponent.Deactivate` (`self.ParticleSystem`)))

(fn `UserConstructionScript`)